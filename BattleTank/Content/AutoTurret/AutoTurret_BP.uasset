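; AutoTurret_BP is an automated turret that sets up its aiming and health bar on BeginPlay.
; It passes its barrel and dome components to the TankAiming component's Initialize.
; It then casts its widget component's user widget to HealthBar and gives that widget a reference to itself.
; Tick and overlap events are disabled, so no per-frame or targeting logic lives in this graph.
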(event EventBeginPlay
  (Class|TankAimingComponent|Initialize (Variables|Default|GetTankAiming) (Variables|Default|GetTurretBarrel) (Variables|Default|GetTurretDome))
  (CallFunction|InitializeHealthBar))

(event Collision|EventActorBeginOverlap
  (params (OtherActor :type Actor%20Object%20Reference)))

(event EventTick
  (params (DeltaSeconds :type Float%20%28single-precision%29)))

(fn ConstructionScript)

(fn InitializeHealthBar
  (bind _ashealth_bar (Utilities|Casting|CastToHealthBar (UserInterface|GetUserWidgetObject (Variables|Default|GetWidget))))
  (Variables|/Game/UI/HealthBar.HealthBar_C|SetAutoTurretRef _ashealth_bar self))